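; Test player character that adds keyboard/mouse Enhanced Input on possession and handles basic move and look.
; Debug keys exercise the camera: X toggles instant focus on a fixed point through ProceduralCameraManager.
; Right mouse toggles a temporary aim, with a timeline driving target vision point and camera distance forward or back.
; The jump action grows the actor's scale instead of jumping, and Z resets it.
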(event Input|EnhancedActionEvents|EnhancedInputActionIA_Look
  (params (ActionValue :type Vector%202D%20Structure) (ElapsedSeconds :type Float%20%28double-precision%29) (TriggeredSeconds :type Float%20%28double-precision%29) (InputAction :type Input%20Action%20Object%20Reference :default "/Game/TestProject/Core/Input/Actions/IA_Look.IA_Look"))
  (bind (_x _y) (Math|Vector2D|BreakVector2D ActionValue))
  (Pawn|Input|AddControllerYawInput _x)
  (Pawn|Input|AddControllerPitchInput _y))

(event Input|EnhancedActionEvents|EnhancedInputActionIA_Move
  (params (ActionValue :type Vector%202D%20Structure) (ElapsedSeconds :type Float%20%28double-precision%29) (TriggeredSeconds :type Float%20%28double-precision%29) (InputAction :type Input%20Action%20Object%20Reference :default "/Game/TestProject/Core/Input/Actions/IA_Move.IA_Move"))
  (bind (_x _y) (Math|Vector2D|BreakVector2D ActionValue))
  (Pawn|Input|AddMovementInput (Transformation|GetActorRightVector) _x false)
  (Pawn|Input|AddMovementInput (Transformation|GetActorForwardVector) _y false))

(event Input|EnhancedActionEvents|EnhancedInputActionIA_Jump
  (params (ActionValue :type Boolean) (ElapsedSeconds :type Float%20%28double-precision%29) (TriggeredSeconds :type Float%20%28double-precision%29) (InputAction :type Input%20Action%20Object%20Reference :default "/Game/TestProject/Core/Input/Actions/IA_Jump.IA_Jump"))
  (Transformation|SetActorScale3D (+ (Transformation|GetActorScale3D) "0.010000,0.010000,0.010000")))

(event EventBeginPlay)

(event Collision|EventActorBeginOverlap
  (params (OtherActor :type Actor%20Object%20Reference)))

(event EventTick
  (params (DeltaSeconds :type Float%20%28single-precision%29)))

(event EventPossessed
  (params (NewController :type Controller%20Object%20Reference))
  (bind _asplayer_controller (Utilities|Casting|CastToPlayerController NewController))
  (Input|AddMappingContext (PlayerController|LocalPlayerSubsystems|GetEnhancedInputLocalPlayerSubsystem _asplayer_controller) "/Game/TestProject/Core/Input/Mappings/IMC_KBM.IMC_KBM" 0 "(bIgnoreAllPressedKeysUntilRelease=True,bForceImmediately=False,bNotifyUserSettings=False)"))

(event Input|MouseEvents|RightMouseButton
  (params (Key :type Key%20Structure :default "None"))
  (:Pressed
    ;[1 1 1] Временное решение
    (Utilities|FlowControl|FlipFlop
      (:A
        (bind (_direction _targetpoint _distance) (Timeline|TL_Aim Play)
          (:Update
            (Class|TestCharacter|SetTargetVisionPoint _targetpoint)
            (Class|TestCharacter|SetDistanceCamerafromTargetVisionPoint _distance))))
      (:B
        (Timeline|TL_Aim Reverse)))))

(event Input|KeyboardEvents|Z
  (params (Key :type Key%20Structure :default "None"))
  (:Pressed
    (Transformation|SetActorScale3D "1.000000,1.000000,1.000000")))

(event Input|KeyboardEvents|X
  (params (Key :type Key%20Structure :default "None"))
  (bind _returnvalue (Game|GetPlayerCameraManager 0))
  (:Pressed
    (Utilities|FlowControl|FlipFlop
      (:A
        (bind _asprocedural_camera_manager (Utilities|Casting|CastToProceduralCameraManager _returnvalue))
        (Class|ProceduralCameraManager|FocusatPoint _asprocedural_camera_manager (Math|Vector|MakeVector 9.1e+02 1e+02 1e+02) true))
      (:B
        (bind _asprocedural_camera_manager_2 (Utilities|Casting|CastToProceduralCameraManager _returnvalue))
        (Class|ProceduralCameraManager|Unfocus _asprocedural_camera_manager_2 true)))))

(fn ConstructionScript)