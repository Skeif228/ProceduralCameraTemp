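; Test player controller that switches the procedural camera behavior according to the type of pawn it possesses.
; On BeginPlay it constructs and stores separate behavior objects for player character, vehicle and FPS cameras.
; On Possess it casts the pawn to TestCharacter, TestVehicle or BP_DefaultPawnFPS and assigns the matching behavior to the ProceduralCameraManager.
; An author note marks this Blueprint setup as a temporary test solution better suited to C++.
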(event EventBeginPlay
  ;[1 1 1] Временное решение. Конечно же лучше все реализовать в C++, но в тесте не так важно
  (bind _returnvalue (Game|ConstructObjectfromClass "/Script/ProceduralCameraTemp.ProceduralPlayerCameraBehavior"))
  (Variables|Default|SetPlayerProceduralCameraBehavior _returnvalue)
  (bind _returnvalue_2 (Game|ConstructObjectfromClass "/Game/ProceduralCamera/Core/CameraBehaviors/BP_ProceduralVehicleCameraBeh.BP_ProceduralVehicleCameraBeh_C"))
  (Variables|Default|SetVehicleProceduralCameraBehavior _returnvalue_2)
  (bind _returnvalue_3 (Game|ConstructObjectfromClass "/Script/ProceduralCameraTemp.ProceduralFPSCameraBehavior"))
  (Variables|Default|SetFPSProceduralCameraBehavior _returnvalue_3))

(event EventPossess
  (params (PossessedPawn :type Pawn%20Object%20Reference))
  (bind _asprocedural_camera_manager (Utilities|Casting|CastToProceduralCameraManager (Game|GetPlayerCameraManager 0)))
  (Utilities|Casting|CastToTestCharacter PossessedPawn
    (:then
      (Variables|/Script/ProceduralCameraTemp.ProceduralCameraManager|SetProceduralCameraBehavior _asprocedural_camera_manager (Variables|Default|GetPlayerProceduralCameraBehavior)))
    (:CastFailed
      (Utilities|Casting|CastToTestVehicle PossessedPawn
        (:then
          (Variables|/Script/ProceduralCameraTemp.ProceduralCameraManager|SetProceduralCameraBehavior _asprocedural_camera_manager (Variables|Default|GetVehicleProceduralCameraBehavior)))
        (:CastFailed
          (Utilities|Casting|CastToBP_DefaultPawnFPS PossessedPawn)
          (Variables|/Script/ProceduralCameraTemp.ProceduralCameraManager|SetProceduralCameraBehavior _asprocedural_camera_manager (Variables|Default|GetFPSProceduralCameraBehavior)))))))

(fn ConstructionScript)